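; Water puzzle actor for the water carriage that rises as the player enters valve combinations, then spawns a doll.
; CheckForCorrectInput matches each valve number against the current level's sequence; mistakes reset progress, play a scare sound and raise player heart rate.
; Completed sequences scale the water up, and the first two also spawn whispering clue notes.
; Tick watches for the maximum level and spawns the doll through a DoOnce.
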(event `self.ReceiveBeginPlay`
  ;[0 0.02214 1] First person character
  (bind _asbp_first_person_character (cast `/Game/FirstPerson/Blueprints/BP_FirstPersonCharacter` (`GameplayStatics.GetPlayerCharacter` 0)))
  (set `self.As BP First Person Character` _asbp_first_person_character))

(event `self.ReceiveTick`
  (params (DeltaSeconds :type "Float (single-precision)"))
  (bind _returnvalue_location (`KismetMathLibrary.BreakTransform` (`SceneComponent.K2_GetComponentToWorld` (`self.Spawnpoint`))))
  ;[0.01818 1 0] Checks if water has reached maximium level and spawns doll
  (if (not (!= (`self.WaterLevel`) 3))
    (`/Engine/EditorBlueprintResources/StandardMacros.DoOnce` false
      (:`Completed`
        (`|SpawnActorFromClass` (`self.SpawnedObject`) (`KismetMathLibrary.Conv_VectorToTransform` _returnvalue_location) "Undefined" "MultiplyWithRoot" null null)
        (`KismetSystemLibrary.PrintString` "DOLL SPAWNED")))))

(event `Rise Water`
  ;[0 0.955 1] Rise water Level until it hits level 3
  (`GameplayStatics.PlaySoundAtLocation` "/Game/Sounds/WaterSlosh.WaterSlosh" (0.0 0.0 0.0) (struct) 1.0 1.0 0.0 null null null null)
  (if (!= (`self.WaterLevel`) 3)
    (`self.SetActorRelativeScale3D` (+ (`self.GetActorScale3D`) (0.0 0.0 0.12)))
    (set `self.WaterLevel` (+ (`self.WaterLevel`) 1))))

(fn `CheckForCorrectInput`
  (params (`Valve Number` :type Integer))
  (bind _as_bp_first_person_character (`self.As BP First Person Character`))
  (bind _as_bp_first_person_character_2 (`self.As BP First Person Character`))
  (bind _as_bp_first_person_character_3 (`self.As BP First Person Character`))
  ;[0 0.9484 1] Checks first combo
  (if (== (`self.WaterLevel`) 0)
    (if (== `Valve Number` (`|GetArrayItem` (`self.CorrectSequence1`) (`self.Index`)))
      (if (== (`self.Index`) 3)
        (`KismetSystemLibrary.PrintString` "Entire combination correct")
        (set `self.Index` 0)
        (`self.Rise Water`)
        (bind _returnvalue (`|SpawnActorFromClass` "/Game/WaterCarriage/Pool_Carriage_Note2.Pool_Carriage_Note2_C" (`self.Note2Transform`) "Undefined" "MultiplyWithRoot" null null))
        (set `self.Note 2` _returnvalue)
        (`GameplayStatics.PlaySoundAtLocation` "/Game/Sounds/Whispers.Whispers" (`SceneComponent.K2_GetComponentLocation` (`Actor.RootComponent` (`self.Note 2`))) (struct) 1.0 1.0 0.0 null null null null)
        (else
          (set `self.Index` (+ (`self.Index`) 1))
          (`KismetSystemLibrary.PrintString` "Correct Input")))
      (else
        (set `self.Index` 0)
        (`GameplayStatics.PlaySound2D` "/Game/Sounds/ScaryErrorNoise.ScaryErrorNoise" 1.0 1.0 0.0 null null)
        (`KismetSystemLibrary.PrintString` "Incorrect Input")
        (set `/Game/FirstPerson/Blueprints/BP_FirstPersonCharacter.Heart Rate` (+ (`/Game/FirstPerson/Blueprints/BP_FirstPersonCharacter.Heart Rate` _as_bp_first_person_character_2) 30.0) _as_bp_first_person_character_2)))
    (elif (== (`self.WaterLevel`) 1)
      ;[0 1 0.4115] Checks if second Combo Is Correct
      (if (== `Valve Number` (`|GetArrayItem` (`self.CorrectSequence2`) (`self.Index`)))
        (if (== (`self.Index`) 3)
          (`KismetSystemLibrary.PrintString` "Entire combination correct")
          (set `self.Index` 0)
          (`self.Rise Water`)
          (bind _returnvalue_2 (`|SpawnActorFromClass` "/Game/WaterCarriage/Pool_Carriage_Note3.Pool_Carriage_Note3_C" (`self.Note3Transform`) "Undefined" "MultiplyWithRoot" null null))
          (set `self.Note 3` _returnvalue_2)
          (`GameplayStatics.PlaySoundAtLocation` "/Game/Sounds/Whispers.Whispers" (`SceneComponent.K2_GetComponentLocation` (`Actor.RootComponent` (`self.Note 3`))) (struct) 1.0 1.0 0.0 null null null null)
          (else
            (set `self.Index` (+ (`self.Index`) 1))
            (`KismetSystemLibrary.PrintString` "Correct Input")))
        (else
          (set `self.Index` 0)
          (`GameplayStatics.PlaySound2D` "/Game/Sounds/ScaryErrorNoise.ScaryErrorNoise" 1.0 1.0 0.0 null null)
          (`KismetSystemLibrary.PrintString` "Incorrect Input")
          (set `/Game/FirstPerson/Blueprints/BP_FirstPersonCharacter.Heart Rate` (+ (`/Game/FirstPerson/Blueprints/BP_FirstPersonCharacter.Heart Rate` _as_bp_first_person_character_3) 30.0) _as_bp_first_person_character_3)))
      (else
        ;[0.2927 1 0] Checks if third combo is correct
        (if (== `Valve Number` (`|GetArrayItem` (`self.CorrectSequence3`) (`self.Index`)))
          (if (== (`self.Index`) 3)
            (`KismetSystemLibrary.PrintString` "Entire combination correct")
            (set `self.Index` 0)
            (`self.Rise Water`)
            (else
              (set `self.Index` (+ (`self.Index`) 1))
              (`KismetSystemLibrary.PrintString` "Correct Input")))
          (else
            (set `self.Index` 0)
            (`GameplayStatics.PlaySound2D` "/Game/Sounds/ScaryErrorNoise.ScaryErrorNoise" 1.0 1.0 0.0 null null)
            (`KismetSystemLibrary.PrintString` "Incorrect Input")
            (set `/Game/FirstPerson/Blueprints/BP_FirstPersonCharacter.Heart Rate` (+ (`/Game/FirstPerson/Blueprints/BP_FirstPersonCharacter.Heart Rate` _as_bp_first_person_character) 30.0) _as_bp_first_person_character)))))))

(fn `UserConstructionScript`)