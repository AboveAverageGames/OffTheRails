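; BP_Camera is a hazard camera that periodically photographs the area ahead, hurting the player if caught in the shot.
; A Delay on Tick paces TakePhoto, which briefly flashes the SpotLight with a sound and box-traces along its forward vector.
; Hitting the first-person character raises its heart rate, pulses HeartRateRaised across one tick, shows a message widget and plays a damage sound.
; Debug trace drawing and hit-name printing remain enabled.
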(event `self.ReceiveBeginPlay`
  ;[0 0.4828 1] Begin play
  (bind _asbp_first_person_character (cast `/Game/FirstPerson/Blueprints/BP_FirstPersonCharacter` (`GameplayStatics.GetPlayerCharacter` 0)))
  (set `self.As BP First Person Character` _asbp_first_person_character))

(event `self.ReceiveTick`
  (params (DeltaSeconds :type "Float (single-precision)"))
  ;[0.08961 1 0] Tick for taking Photo
  (set `self.TakingPhoto` false)
  (`KismetSystemLibrary.Delay` (`self.PhotoDelay`))
  (bind _output_get (set `self.TakingPhoto` true))
  (if _output_get
    (`self.TakePhoto`)))

(event `TakePhoto`
  (bind _spotlight (`self.SpotLight`))
  (bind _as_bp_first_person_character (`self.As BP First Person Character`))
  (bind _returnvalue (`SceneComponent.K2_GetComponentLocation` _spotlight))
  ;[1 0.006282 0] Take Photo Event
  (`GameplayStatics.PlaySoundAtLocation` "/Game/Sounds/CameraFlash2.CameraFlash2" _returnvalue (struct) 1.0 1.0 0.0 null null null null)
  (`SceneComponent.SetVisibility` (`self.SpotLight`) true true)
  (bind _outhit (`KismetSystemLibrary.BoxTraceSingle` :`Start` (+ _returnvalue (0.0 -70.0 25.0)) :`End` (+ _returnvalue (* (`KismetMathLibrary.GetForwardVector` (`SceneComponent.K2_GetComponentRotation` _spotlight)) (`self.CameraRange`))) :`HalfSize` (60.0 60.0 60.0) :`TraceChannel` "TraceTypeQuery3" :`DrawDebugType` "ForDuration"))
  (bind (_bblockinghit _binitialoverlap _time _distance _location _impactpoint _normal _impactnormal _physmat _hitactor) (`GameplayStatics.BreakHitResult` _outhit))
  (`KismetSystemLibrary.PrintString` (`KismetSystemLibrary.GetDisplayName` _hitactor))
  (if (== (`self.As BP First Person Character`) _hitactor)
    ;[1 0.39 0] Increases heart rate when spotted
    (set `/Game/FirstPerson/Blueprints/BP_FirstPersonCharacter.Heart Rate` (+ (`/Game/FirstPerson/Blueprints/BP_FirstPersonCharacter.Heart Rate` _as_bp_first_person_character) (`self.HeartRateIncreasedBy`)) _as_bp_first_person_character)
    (set `/Game/FirstPerson/Blueprints/BP_FirstPersonCharacter.HeartRateRaised` false _as_bp_first_person_character)
    (`KismetSystemLibrary.DelayUntilNextTick`)
    (set `/Game/FirstPerson/Blueprints/BP_FirstPersonCharacter.HeartRateRaised` true _as_bp_first_person_character)
    (bind _returnvalue_2 (`|CreateWidget` "/Game/Widgets/WB_ItemPickedUpMessage.WB_ItemPickedUpMessage_C"))
    (set `/Game/Widgets/WB_ItemPickedUpMessage.ItemPickedUP` "They captured a picture of me.. It hurts.." _returnvalue_2)
    (`UserWidget.AddToViewport` _returnvalue_2 0)
    (`GameplayStatics.PlaySound2D` "/Game/Sounds/DamageTaken.DamageTaken" 1.0 1.0 0.0 null null))
  (`KismetSystemLibrary.Delay` 0.2)
  (`SceneComponent.SetVisibility` (`self.SpotLight`) false true))

(fn `UserConstructionScript`)