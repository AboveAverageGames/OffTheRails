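; Door actor in the Western carriage that takes the player to the Pool_Carriage level on interaction.
; When the player character enters InteractableCollision, it shows a WB_EToInteract prompt and enables input on the door.
; Leaving the collision removes the prompt and disables input, so IA_Interact is meant to trigger the level change only in range.
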(event `self.Interactable Collision.OnComponentBeginOverlap`
  (params (OverlappedComponent :type "PrimitiveComponent Object Reference") (OtherActor :type "Actor Object Reference") (OtherComp :type "PrimitiveComponent Object Reference") (OtherBodyIndex :type Integer) (bFromSweep :type Boolean) (SweepResult :type "HitResult Structure (by ref)"))
  (bind _returnvalue (`GameplayStatics.GetPlayerCharacter` 0))
  ;[0 1 0.07119] Interact Widget Show
  (bind _output_get (set `self.Other Actor` OtherActor))
  (if (== _output_get _returnvalue)
    (bind _asbp_first_person_character (cast `/Game/FirstPerson/Blueprints/BP_FirstPersonCharacter` _returnvalue))
    (set `self.Player Controller` (`PlayerState.GetPlayerController` (`Pawn.PlayerState` _asbp_first_person_character)))
    (bind _returnvalue_2 (`|CreateWidget` "/Game/Widgets/WB_EToInteract.WB_EToInteract_C"))
    (bind _output_get_2 (set `self.WB_Interact` _returnvalue_2))
    (`UserWidget.AddToViewport` _output_get_2 0)
    (`self.EnableInput` (`self.Player Controller`))))

(event `self.Interactable Collision.OnComponentEndOverlap`
  (params (OverlappedComponent :type "PrimitiveComponent Object Reference") (OtherActor :type "Actor Object Reference") (OtherComp :type "PrimitiveComponent Object Reference") (OtherBodyIndex :type Integer))
  ;[1 0 0.04771] Remove Interact Widget
  (bind _output_get (set `self.Other Actor` OtherActor))
  (if (== _output_get (`GameplayStatics.GetPlayerCharacter` 0))
    (`Widget.RemoveFromParent` (`self.WB_Interact`))
    (`self.DisableInput` (`self.Player Controller`))))

(event `EnhancedInput|/Game/FirstPerson/Input/Actions/IA_Interact`
  (params (ActionValue :type Boolean) (ElapsedSeconds :type "Float (double-precision)") (TriggeredSeconds :type "Float (double-precision)") (InputAction :type "InputAction Object Reference" :default "/Game/FirstPerson/Input/Actions/IA_Interact.IA_Interact"))
  ;[1 0.9015 0] On Interact
  (:`Started`
    (`GameplayStatics.OpenLevelBySoftObjectPtr` "/Game/levels/Pool_Carriage.Pool_Carriage")))

(fn `UserConstructionScript`)